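; Mod Blueprint that keeps a count-up timer for the action phase of a heist.
; On BeginPlay it binds to the game event broker's action-phase-entered event.
; That event starts a looping timer by function name and adds a UI_HeistTimer widget to the viewport.
; Each timer tick increments Seconds, rolling over into Minutes past 59.
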(event Custom|OnActionPhaseEntered_Event_0
  (Utilities|Time|SetTimerbyFunctionName 0 "bigHeistTimer" 0.0 true)
  (bind _returnvalue (UserInterface|CreateWidget "/Game/Mods/_SanicsMods/HeistTimer/UI_HeistTimer.UI_HeistTimer_C"))
  (UserInterface|Viewport|AddtoViewport _returnvalue 0))

(event Custom|bigHeistTimer
  (Variables|Default|SetSeconds (+ (Variables|Default|GetSeconds) 1))
  (if (> (Variables|Default|GetSeconds) 59)
    (Variables|Default|SetMinutes (+ (Variables|Default|GetMinutes) 1))
    (Variables|Default|SetSeconds 0)))

(event EventBeginPlay
  (|CallParentFunction)
  (bind _returnvalue (Class|SBZEventLibrary|GetGameEventBroker))
  (EventDispatchers|BindEventtoOnActionPhaseEntered _returnvalue (EventDispatchers|CreateEvent :!event Custom|OnActionPhaseEntered_Event_0)))

(fn ConstructionScript
  (|CallParentFunction))

(fn BPHeistTimerAutoGenFunc)