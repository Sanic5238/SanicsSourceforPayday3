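; Mod actor that shows an on-screen notification with a sound whenever a challenge is completed.
; On BeginPlay it binds to the challenge manager's completion event and adds a UI_ChallengeTray widget to the viewport.
; Each completion pushes the challenge's name and description into the tray and posts the Sanic_ChallengeNotifications_Anime Wwise event on the local player controller.
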(event Custom|OnCompletedChallenge_Event_0
  (params (ChallengeData :type SBZ%20Challenge%20Data%20Structure%20%28by%20ref%29))
  (Default|AddNotification (Variables|Default|GetChallenge%20Tray) (Utilities|Text|ToText(String) (.ChallengeName (Utilities|Struct|BreakSBZChallengeData ChallengeData))) (Class|SBZChallengeManager|GetChallengeDescriptionText (Class|SBZChallengeManager|GetChallengeManager) ChallengeData))
  (Class|AkGameplayStatics|PostEvent "/Game/WwiseAudio/Events/Sanic_ChallengeNotifications/Sanic_ChallengeNotifications_Anime.Sanic_ChallengeNotifications_Anime" (Class|SBZPlayerLibrary|GetLocalPlayerController)))

(event EventBeginPlay
  (|CallParentFunction)
  (EventDispatchers|BindEventtoOnCompletedChallenge (Class|SBZChallengeManager|GetChallengeManager) (EventDispatchers|CreateEvent :!event Custom|OnCompletedChallenge_Event_0))
  (bind _returnvalue (UserInterface|CreateWidget "/Game/Mods/_SanicsMods/ChallengeNotifications/UI_ChallengeTray.UI_ChallengeTray_C"))
  (UserInterface|Viewport|AddtoViewport _returnvalue 0)
  (Variables|Default|SetChallenge%20Tray _returnvalue))

(fn ConstructionScript
  (|CallParentFunction))