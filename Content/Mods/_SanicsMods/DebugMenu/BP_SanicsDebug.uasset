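; BP_SanicsDebug is a mod Blueprint that toggles a debug popup menu with the Insert key.
; It creates a UI_DebugPopup widget on BeginPlay, then polls the local player controller on Tick to add or remove it from the viewport.
; Opening the menu also caches a hardcoded challenge from the challenge manager as ArmorChall.
; An unused Rem event would remove that challenge from the completed challenges list.
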(event Custom|Rem
  (bind _returnvalue (Class|SBZChallengeManager|GetChallengeManager))
  (bind _completedchallenges (Variables|/Script/Starbreeze.SBZChallengeManager|GetCompletedChallenges _returnvalue))
  (for (_array_element _array_index) _completedchallenges
    (if (Utilities|Name|Equal(Name) (.ChallengeId (Utilities|Struct|BreakSBZChallengeData _array_element)) (.ChallengeId (Utilities|Struct|BreakSBZChallengeData (Variables|Default|GetArmorChall))))
      (Utilities|Array|RemoveIndex _completedchallenges _array_index))))

(event EventBeginPlay
  (|CallParentFunction)
  (bind _returnvalue (UserInterface|CreateWidget "/Game/Mods/_SanicsMods/DebugMenu/UI_DebugPopup.UI_DebugPopup_C"))
  (Variables|Default|SetDebugMenu _returnvalue))

(event EventTick
  (params (DeltaSeconds :type Float%20%28single-precision%29))
  (bind _debugmenu (Variables|Default|GetDebugMenu))
  (bind _returnvalue (Class|SBZUtilityLibrary|GetLocalPlayerController))
  (if (Game|Player|WasInputKeyJustPressed _returnvalue "Insert")
    (if (Math|Boolean|Equal(Boolean) (Variables|Default|GetisOpen) true)
      (Widget|RemovefromParent _debugmenu)
      (Variables|Default|SetisOpen false)
      (else
        (Variables|Default|SetArmorChall (.Value (Utilities|Map|Find (Variables|/Script/Starbreeze.SBZChallengeManager|GetChallengeMap (Class|SBZChallengeManager|GetChallengeManager)) "63cfc0257f0dd5f341f393cf")))
        (UserInterface|Viewport|AddtoViewport _debugmenu 0)
        (Variables|Default|SetisOpen true)))))

(fn ConstructionScript
  (|CallParentFunction))